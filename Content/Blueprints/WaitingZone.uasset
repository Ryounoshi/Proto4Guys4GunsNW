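; WaitingZone is a holding area that keeps a player until they enter its teleporter into play.
; On the server, AddPlayer moves the player to SpawnPoint, marks the zone occupied and resets the DoOnce gate.
; The first character overlapping Teleporteur after each reset frees the zone on authority, updates that character's state, teleports it to a random PlayerStart and calls StartGame on CountDown.
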(event `self.ReceiveBeginPlay`
  (bind _outactors (`GameplayStatics.GetAllActorsOfClass` "/Script/Engine.PlayerStart"))
  (set `self.SpawnPoints` _outactors))

(event `self.ReceiveActorBeginOverlap`
  (params (OtherActor :type "Actor Object Reference")))

(event `self.ReceiveTick`
  (params (DeltaSeconds :type "Float (single-precision)")))

(event `AddPlayer`
  (params (Player :type "/Game/Blueprints/MyCharacter Object Reference"))
  (`/Engine/EditorBlueprintResources/ActorMacros.Switch Has Authority`
    (:`Authority`
      (`/Engine/EditorBlueprintResources/StandardMacros.IsValid` Player
        (:`Is Valid`
          (`self.ResetGate`)
          (set `self.Free` false)
          (set `/Game/Blueprints/MyCharacter.InWaitingZone` true Player)
          (`self.K2_SetActorLocation` Player (`SceneComponent.K2_GetComponentLocation` (`self.SpawnPoint`)) false true))))))

(event `self.Teleporteur.OnComponentBeginOverlap`
  (params (OtherActor :type "Actor Object Reference") (OtherComp :type "PrimitiveComponent Object Reference") (OtherBodyIndex :type Integer) (bFromSweep :type Boolean) (SweepResult :type "HitResult Structure (by ref)"))
  (bind _spawnpoints (`self.SpawnPoints`))
  (bind _asmy_character (cast `/Game/Blueprints/MyCharacter` OtherActor))
  (`/Engine/EditorBlueprintResources/StandardMacros.DoOnce` true :!label _label
    (:`Completed`
      (`/Engine/EditorBlueprintResources/ActorMacros.Switch Has Authority`
        (:`Authority`
          (set `self.Free` true)
          (set `/Game/Blueprints/MyCharacter.InWaitingZone` false _asmy_character)
          (`/Game/Blueprints/MyCharacter.DisableShadows` _asmy_character true)
          (`/Game/Blueprints/MyCharacter.ClientJoined` _asmy_character)
          (`self.K2_SetActorLocation` _asmy_character (`self.K2_GetActorLocation` (`KismetArrayLibrary.Array_Get` _spawnpoints (`KismetMathLibrary.RandomIntegerInRange` 0 (- (`KismetArrayLibrary.Array_Length` _spawnpoints) 1)))) false true)
          (`/Game/Blueprints/CountDown.StartGame` (`self.CountDown`)))))))

(event `ResetGate`
  (goto _label :!via `Reset`))

(fn `UserConstructionScript`)