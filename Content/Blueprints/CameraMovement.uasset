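; Actor that stages a Star Wars-style intro crawl with prologue, scaling title and scrolling team credits, snapping the camera to itself on AttachCam.
; PlayGeneric chains timelines and delays with theme music, then opens a Tick gate that moves the text and lets GameManager's Enter flag trigger game entry.
; After a timeout without Enter, StopGeneric fades out music and screen, hides everything and closes the gate, then CutScene1 plays.
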(event `AttachCam`
  (`self.K2_AttachRootComponentToActor` (`self.Camera`) self "None" "SnapToTarget" true))

(event `self.ReceiveActorBeginOverlap`
  (params (OtherActor :type "Actor Object Reference")))

(event `self.ReceiveBeginPlay`)

(event `self.ReceiveTick`
  (params (DeltaSeconds :type "Float (single-precision)"))
  (`/Engine/EditorBlueprintResources/StandardMacros.Gate` true :!label _label
    (:`Exit`
      (`SceneComponent.K2_AddRelativeLocation` (`self.Vincent`) (* (* (`KismetMathLibrary.MakeVector` 0.2 0.0 0.06) 0.26) (* DeltaSeconds 60.0)) false true)
      (`SceneComponent.K2_AddRelativeLocation` (`self.Timothe`) (* (* (`KismetMathLibrary.MakeVector` 0.2 0.0 0.06) 0.26) (* DeltaSeconds 60.0)) false true)
      (`SceneComponent.K2_AddRelativeLocation` (`self.Louis`) (* (* (`KismetMathLibrary.MakeVector` 0.2 0.0 0.06) 0.26) (* DeltaSeconds 60.0)) false true)
      (`SceneComponent.K2_AddRelativeLocation` (`self.Graphistes`) (* (* (`KismetMathLibrary.MakeVector` 0.2 0.0 0.06) 0.26) (* DeltaSeconds 60.0)) false true)
      (`SceneComponent.K2_AddRelativeLocation` (`self.LevelDesigner`) (* (* (`KismetMathLibrary.MakeVector` 0.2 0.0 0.06) 0.26) (* DeltaSeconds 60.0)) false true)
      (`SceneComponent.K2_AddRelativeLocation` (`self.Nicolas`) (* (* (`KismetMathLibrary.MakeVector` 0.2 0.0 0.06) 0.26) (* DeltaSeconds 60.0)) false true)
      (`SceneComponent.K2_AddRelativeLocation` (`self.Adilson`) (* (* (`KismetMathLibrary.MakeVector` 0.2 0.0 0.06) 0.26) (* DeltaSeconds 60.0)) false true)
      (`SceneComponent.K2_AddRelativeLocation` (`self.Programmer`) (* (* (`KismetMathLibrary.MakeVector` 0.2 0.0 0.06) 0.26) (* DeltaSeconds 60.0)) false true)
      (`SceneComponent.K2_AddRelativeLocation` (`self.Rudi`) (* (* (`KismetMathLibrary.MakeVector` 0.2 0.0 0.06) 0.26) (* DeltaSeconds 60.0)) false true)
      (`SceneComponent.K2_AddRelativeLocation` (`self.TextRender5`) (* (* (`KismetMathLibrary.MakeVector` 0.2 0.0 0.06) 0.26) (* DeltaSeconds 60.0)) false true)
      (`SceneComponent.K2_AddRelativeLocation` (`self.TextRender1`) (* (* (`KismetMathLibrary.MakeVector` 0.2 0.0 0.06) 0.26) (* DeltaSeconds 60.0)) false true)
      (`SceneComponent.K2_AddRelativeLocation` (`self.TextRender2`) (* (* (`KismetMathLibrary.MakeVector` 0.2 0.0 0.06) 0.26) (* DeltaSeconds 60.0)) false true)
      (`SceneComponent.K2_AddRelativeLocation` (`self.TextRender3`) (* (* (`KismetMathLibrary.MakeVector` 0.2 0.0 0.06) 0.26) (* DeltaSeconds 60.0)) false true)
      (`SceneComponent.K2_AddRelativeLocation` (`self.TextRender4`) (* (* (`KismetMathLibrary.MakeVector` 0.2 0.0 0.06) 0.26) (* DeltaSeconds 60.0)) false true)
      (`SceneComponent.K2_AddRelativeLocation` (`self.TextRender`) (* (* (`KismetMathLibrary.MakeVector` 0.2 0.0 0.06) 0.26) (* DeltaSeconds 60.0)) false true)
      (`SceneComponent.K2_AddRelativeLocation` (`self.TextRender6`) (* (* (`KismetMathLibrary.MakeVector` 0.2 0.0 0.06) 0.26) (* DeltaSeconds 60.0)) false true)
      (`SceneComponent.K2_AddRelativeLocation` (`self.TextRender7`) (* (* (`KismetMathLibrary.MakeVector` 0.2 0.0 0.06) 0.26) (* DeltaSeconds 60.0)) false true)
      (`SceneComponent.K2_AddRelativeLocation` (`self.TextRender8`) (* (* (`KismetMathLibrary.MakeVector` 0.2 0.0 0.06) 0.26) (* DeltaSeconds 60.0)) false true)
      (`SceneComponent.K2_AddRelativeLocation` (`self.TextRender9`) (* (* (`KismetMathLibrary.MakeVector` 0.2 0.0 0.06) 0.26) (* DeltaSeconds 60.0)) false true)
      (`SceneComponent.K2_AddRelativeLocation` (`self.TextRender10`) (* (* (`KismetMathLibrary.MakeVector` 0.2 0.0 0.06) 0.26) (* DeltaSeconds 60.0)) false true)
      (`SceneComponent.K2_AddRelativeLocation` (`self.TextRender11`) (* (* (`KismetMathLibrary.MakeVector` 0.2 0.0 0.06) 0.26) (* DeltaSeconds 60.0)) false true)
      (if (`/Game/Blueprints/Managers/GameManager.EnterPushed` (`self.GameManager`))
        (`/Engine/EditorBlueprintResources/StandardMacros.DoOnce` false
          (:`Completed`
            (`/Game/Blueprints/Managers/GameManager.TryToEnterInGame` (`self.GameManager`))))))))

(event `PlayGeneric`
  (bind _titre (`self.Titre`))
  (bind _star_wars_theme_cue (`self.star_wars_theme_Cue`))
  (set `self.GenericIsPlaying` true)
  (`MatineeActor.Play` (`self.FadeFromBlack`))
  (`SceneComponent.SetVisibility` (`self.StaticMesh`) true false)
  (`SceneComponent.SetVisibility` (`self.Cube`) true false)
  (`SceneComponent.SetVisibility` (`self.Prologue`) true false)
  (`KismetSystemLibrary.Delay` 4.0)
  (bind (_direction _newtrack_0) (`Timeline|Fade` :!via `PlayFromStart`)
    (:`Update`
      (`MaterialInstanceDynamic.SetScalarParameterValue` (`self.Mat`) "Opacity" _newtrack_0))
    (:`Finished`
      (`KismetSystemLibrary.Delay` 2.0)
      (`AudioComponent.Stop` _star_wars_theme_cue)
      (`AudioComponent.SetVolumeMultiplier` _star_wars_theme_cue 1.0)
      (`AudioComponent.Play` _star_wars_theme_cue 0.0)
      (`SceneComponent.SetVisibility` (`self.Titre`) true false)
      (`|ExecutionSequence`
        (:`then_0`
          (bind (_direction_2 _newtrack_0_2) (`Timeline|Scale` :!via `PlayFromStart`)
            (:`Update`
              (`SceneComponent.SetWorldScale3D` _titre (`KismetMathLibrary.MakeVector` _newtrack_0_2 _newtrack_0_2 _newtrack_0_2)))
            (:`Finished`
              (`SceneComponent.SetVisibility` _titre false false))))
        (:`then_1`
          (`|ExecutionSequence`
            (:`then_0`
              (goto _label :!via `Open`))
            (:`then_1`
              (`KismetSystemLibrary.Delay` 52.0)
              (if (not (`/Game/Blueprints/Managers/GameManager.EnterPushed` (`self.GameManager`)))
                (`self.StopGeneric`)
                (`KismetSystemLibrary.Delay` 1.0)
                (`MatineeActor.Play` (`self.CutScene1`))))))))))

(event `StopGeneric`
  (bind _star_wars_theme_cue (`self.star_wars_theme_Cue`))
  (if (`self.GenericIsPlaying`)
    (set `self.GenericIsPlaying` false)
    (`|ExecutionSequence`
      (:`then_0`
        (bind (_direction _newtrack_1) (`Timeline|SoundPower` :!via `PlayFromStart`)
          (:`Update`
            (`AudioComponent.SetVolumeMultiplier` _star_wars_theme_cue _newtrack_1))
          (:`Finished`
            (`AudioComponent.Stop` _star_wars_theme_cue))))
      (:`then_1`
        (`MatineeActor.Play` (`self.FadeToBlack`))
        (`KismetSystemLibrary.Delay` 0.6)
        (`SceneComponent.SetVisibility` (`self.Vincent`) false false)
        (`SceneComponent.SetVisibility` (`self.Timothe`) false false)
        (`SceneComponent.SetVisibility` (`self.Louis`) false false)
        (`SceneComponent.SetVisibility` (`self.Graphistes`) false false)
        (`SceneComponent.SetVisibility` (`self.LevelDesigner`) false false)
        (`SceneComponent.SetVisibility` (`self.Nicolas`) false false)
        (`SceneComponent.SetVisibility` (`self.Adilson`) false false)
        (`SceneComponent.SetVisibility` (`self.Programmer`) false false)
        (`SceneComponent.SetVisibility` (`self.Rudi`) false false)
        (`SceneComponent.SetVisibility` (`self.Titre`) false false)
        (`SceneComponent.SetVisibility` (`self.TextRender5`) false false)
        (`SceneComponent.SetVisibility` (`self.TextRender1`) false false)
        (`SceneComponent.SetVisibility` (`self.TextRender2`) false false)
        (`SceneComponent.SetVisibility` (`self.TextRender3`) false false)
        (`SceneComponent.SetVisibility` (`self.TextRender4`) false false)
        (`SceneComponent.SetVisibility` (`self.TextRender`) false false)
        (`SceneComponent.SetVisibility` (`self.TextRender6`) false false)
        (`SceneComponent.SetVisibility` (`self.TextRender7`) false false)
        (`SceneComponent.SetVisibility` (`self.TextRender8`) false false)
        (`SceneComponent.SetVisibility` (`self.TextRender9`) false false)
        (`SceneComponent.SetVisibility` (`self.TextRender10`) false false)
        (`SceneComponent.SetVisibility` (`self.TextRender11`) false false)
        (`SceneComponent.SetVisibility` (`self.Prologue`) false false)
        (`SceneComponent.SetVisibility` (`self.StaticMesh`) false false)
        (`SceneComponent.SetVisibility` (`self.Cube`) false false)
        (goto _label :!via `Close`)))))

(fn `UserConstructionScript`
  (bind _returnvalue (`PrimitiveComponent.CreateDynamicMaterialInstance` (`self.Prologue`) 0 "/Game/Effects/Materials/TextUnlite.TextUnlite"))
  (set `self.Mat` _returnvalue))