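; CountDown is the match timer actor that starts, runs and ends an arena round, with countdown and score widgets.
; The authority starts it once two players join, then uses a Delay in Tick to count down each second, popping a platform every 45 seconds.
; At zero it triggers cinematic mode, shows up to eight players' scores unless CameraMovement is playing, then resets the game.
; A score bubble sort is present but disconnected.
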(event `PlayJoinSoundMulticast`
  (if (not (`/Game/Blueprints/CameraMovement.GenericIsPlaying` (`self.CameraMovement`)))
    (`GameplayStatics.PlaySound2D` "/Game/Son/PlayerJoined.PlayerJoined" 0.8 1.0 0.0)))

(event `PlayJoinSound`
  (`self.PlayJoinSoundMulticast`))

(event `PlayEndSound`
  (if (not (`/Game/Blueprints/CameraMovement.GenericIsPlaying` (`self.CameraMovement`)))
    (`GameplayStatics.PlaySound2D` "/Game/Son/GameFinished.GameFinished" 0.5)))

(event `self.ReceiveBeginPlay`
  (`/Engine/EditorBlueprintResources/ActorMacros.Switch Has Authority`
    (:`Authority`
      (bind _outactors (`GameplayStatics.GetAllActorsOfClass` "/Game/Blueprints/Managers/MyGameMode.MyGameMode_C"))
      (set `self.GameMode` (`KismetArrayLibrary.Array_Get` _outactors))
      (set `self.GameTime` (`self.MaxGameTime`)))))

(event `PlayStartSound`
  (if (not (`/Game/Blueprints/CameraMovement.GenericIsPlaying` (`self.CameraMovement`)))
    (`GameplayStatics.PlaySound2D` "/Game/Son/StartGame.StartGame" 0.5)))

(event `StartGame`
  (`/Engine/EditorBlueprintResources/ActorMacros.Switch Has Authority`
    (:`Authority`
      (bind _result (`/Engine/EditorBlueprintResources/StandardMacros.IncrementInt` (`self.NumberOfPlayerJoinedArena`))
        (:`  `
          (if (and (not (`self.GameStarted`)) (>= _result 2))
            (set `self.GameStarted` true)
            (`self.PlayStartSound`)))))))

(event `UpdateTime`
  (bind _countdownwidget (`self.CountDownWidget`))
  (`/Engine/EditorBlueprintResources/StandardMacros.IsValid` _countdownwidget
    (:`Is Valid`
      (`/Game/Blueprints/Widgets/CountDownWidget.SetTime` _countdownwidget (`KismetTextLibrary.Conv_IntToText` (`self.GameTime`))))))

(event `self.ReceiveActorBeginOverlap`
  (params (OtherActor :type "Actor Object Reference")))

(event `self.ReceiveTick`
  (params (DeltaSeconds :type "Float (single-precision)"))
  (bind _gametime (`self.GameTime`))
  (`/Engine/EditorBlueprintResources/ActorMacros.Switch Has Authority`
    (:`Authority`
      (if (`self.GameStarted`)
        (`KismetSystemLibrary.Delay` 1.0)
        (bind _result (`/Engine/EditorBlueprintResources/StandardMacros.DecrementInt` _gametime)
          (:`  `
            (`self.UpdateTime`)
            (if (== (mod _gametime 45) 0)
              (`/Game/Blueprints/Managers/GameManager.PopPlateforme` (`self.GameManager`)))
            (if (<= _result 0)
              (`self.StopGame`))))))))

(event `ShowScore`
  (params (PlayerList :type "Array of /Game/Blueprints/MyCharacter Object Reference"))
  (bind _returnvalue (`|CreateWidget` "/Game/Blueprints/Widgets/ScoreWidget.ScoreWidget_C"))
  (bind _output_get (set `self.ScoreTabWidget` _returnvalue))
  (`/Game/Blueprints/Widgets/ScoreWidget.UpdateListe` _output_get PlayerList)
  (`UserWidget.AddToViewport` _output_get 0))

(event `ShowTime`
  (bind _returnvalue (`|CreateWidget` "/Game/Blueprints/Widgets/CountDownWidget.CountDownWidget_C"))
  (bind _output_get (set `self.CountDownWidget` _returnvalue))
  (`UserWidget.AddToViewport` _output_get 0))

(event `StopGame`
  (bind _playerlist (`self.PlayerList`))
  (set `self.GameStarted` false)
  (`/Game/Blueprints/Managers/MyGameMode.StopGame` (`self.GameMode`))
  (`self.PlayEndSound`)
  (`/Game/Blueprints/ResetManager.GoInCinematicMode` (`self.ResetManager`))
  (set `self.NumberOfPlayerJoinedArena` 0)
  (`KismetArrayLibrary.Array_Clear` _playerlist)
  (for (_array_element _array_index) (`/Game/Blueprints/Managers/MyGameMode.PlayerList` (`self.GameMode`))
    (`/Engine/EditorBlueprintResources/StandardMacros.IsValid` _array_element
      (:`Is Valid`
        (if (< _array_index 8)
          (`KismetArrayLibrary.Array_Add` _playerlist _array_element)))))
  (if (not (`/Game/Blueprints/CameraMovement.GenericIsPlaying` (`self.CameraMovement`)))
    (`self.ShowScore` _playerlist))
  (`KismetSystemLibrary.Delay` 5.0)
  (set `self.GameTime` (`self.MaxGameTime`))
  (`/Game/Blueprints/Managers/MyGameMode.ResetGame` (`self.GameMode`)))

(fn `UserConstructionScript`)